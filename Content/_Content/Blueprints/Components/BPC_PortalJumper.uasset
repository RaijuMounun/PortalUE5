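; BPC_PortalJumper is an actor component that teleports its owner to another portal while preserving its speed.
; Its PortalJump event records the owner's velocity magnitude, then moves it to the supplied target location and rotation.
; It aligns the instigator's control rotation with the target when the instigator is valid.
; Finally, it redirects the saved speed along the new forward vector through the passed-in movement component.
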(event `self.ReceiveBeginPlay`
  (set `self.Owner` (`self.GetOwner`)))

(event `PortalJump`
  (params (TargetLocation :type "Vector Structure") (TargetRotation :type "Rotator Structure") (MovementComponent :type "MovementComponent Object Reference"))
  (bind _instigator (`Actor.Instigator` (`self.Owner`)))
  ;[0.03646 0.03646 0.03646] Get Jump Velocity
  (set `self.JumpVelocity` (`KismetMathLibrary.VSize` (`Actor.GetVelocity` (`self.Owner`))))
  ;[0.03646 0.03646 0.03646] Teleport actor to other portal
  (`Actor.K2_SetActorLocationAndRotation` (`self.Owner`) TargetLocation TargetRotation false false)
  ;[0.03646 0.03646 0.03646] Fix rotation
  (`/Engine/EditorBlueprintResources/StandardMacros.IsValid` _instigator
    (:`Is Valid`
      (`Controller.SetControlRotation` (`Pawn.GetController` _instigator) TargetRotation))
    (:`Is Not Valid`
      _))
  ;[0.03646 0.03646 0.03646] Set Jump Velocity back
  (set `MovementComponent.Velocity` (* (`Actor.GetActorForwardVector` (`self.Owner`)) (`self.JumpVelocity`)) MovementComponent))